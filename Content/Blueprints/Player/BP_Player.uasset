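; Player character that creates the HUD, handles movement and look input, and picks up items with E.
; Pickup messages overlapping BP_Item actors through BPI_Items, then spawns a flashlight or key by item name and attaches it to a socket on ItemInHand.
; Each tick it feeds control rotation to the animation Blueprint as head rotation, smoothly turning the body when the view yaw strays past 90 degrees either side.
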(event EventBeginPlay
  (bind _returnvalue (UserInterface|CreateWidget "/Game/Assets/GUI/WB_HUD.WB_HUD_C"))
  (UserInterface|Viewport|AddtoViewport _returnvalue 0))

(event Collision|EventActorBeginOverlap
  (params (OtherActor :type Actor%20Object%20Reference)))

(event EventTick
  (params (DeltaSeconds :type Float%20%28single-precision%29))
  (Utilities|FlowControl|Sequence
    (:then_0
      (if (not (AI|Components|NavMovement|IsFalling (Variables|Character|GetCharacterMovement)))
        (Variables|Default|SetHasJumped false)))
    (:then_1
      (CallFunction|UpdateHeadPosition))))

(event Input|AxisEvents|InputAxisMoveForwardBackward
  (params (AxisValue :type Float%20%28single-precision%29))
  (Pawn|Input|AddMovementInput (Math|Vector|GetForwardVector (Math|Rotator|MakeRotator 0.0 0.0 (.yaw (Pawn|GetControlRotation :!class /Script/Engine.Pawn)))) AxisValue false))

(event Input|AxisEvents|InputAxisMoveRightLeft
  (params (AxisValue :type Float%20%28single-precision%29))
  (bind _returnvalue (Pawn|GetControlRotation :!class /Script/Engine.Pawn))
  (Pawn|Input|AddMovementInput (Math|Vector|GetRightVector (Math|Rotator|MakeRotator (.roll _returnvalue) 0.0 (.yaw _returnvalue))) AxisValue false))

(event Input|AxisEvents|InputAxisMouseHorizontal
  (params (AxisValue :type Float%20%28single-precision%29))
  (Pawn|Input|AddControllerYawInput AxisValue)
  (Variables|Default|SetTurnRate AxisValue))

(event Input|AxisEvents|InputAxisMouseVertical
  (params (AxisValue :type Float%20%28single-precision%29))
  (Pawn|Input|AddControllerPitchInput AxisValue))

(event Input|KeyboardEvents|E
  (params (Key :type Key%20Structure :default "None"))
  (:Pressed
    (for _array_element (Collision|GetOverlappingActors "/Game/Blueprints/Items/BP_Item.BP_Item_C" :!class /Script/Engine.Actor)
      (if (Utilities|DoesObjectImplementInterface _array_element "/Game/Blueprints/Items/BPI_Items.BPI_Items_C")
        (Class|BPIItems|PickUp(Message) _array_element)
        (bind _asbp_item (Utilities|Casting|CastToBP_Item _array_element))
        (Utilities|FlowControl|Sequence
          (:then_0
            (if (Utilities|Enum|Equal(Enum) "flashlight" (Variables|/Game/Blueprints/Items/BP_Item.BP_Item_C|GetName _asbp_item))
              (bind _returnvalue (Game|SpawnActorfromClass "/Game/Blueprints/Flashlight/BP_Flashlight.BP_Flashlight_C" (Transformation|GetSocketTransform (Variables|Default|GetItemInHand) "SocketFlashlight" "RTS_World") "Undefined" 0 0))
              (Transformation|AttachComponentToComponent _returnvalue (Variables|Default|GetItemInHand) "SocketFlashlight" "SnapToTarget" "SnapToTarget" "SnapToTarget" true)
              (Variables|Default|SetHasFlahlight true)))
          (:then_1
            (if (Utilities|Enum|Equal(Enum) "key" (Variables|/Game/Blueprints/Items/BP_Item.BP_Item_C|GetName _asbp_item))
              (bind _returnvalue_2 (Game|SpawnActorfromClass "/Game/Blueprints/Key/BP_Key.BP_Key_C" (Transformation|GetSocketTransform (Variables|Default|GetItemInHand) "SocketKey" "RTS_World") "Undefined" 0 0))
              (Transformation|AttachComponentToComponent _returnvalue_2 (Variables|Default|GetItemInHand) "SocketKey" "SnapToTarget" "SnapToTarget" "SnapToTarget" true))))))))

(fn ConstructionScript)

(fn UpdateHeadPosition
  (bind _returnvalue (Pawn|GetControlRotation :!class /Script/Engine.Pawn))
  (bind _returnvalue_2 (Transformation|GetActorRotation))
  (bind _returnvalue_3 (- (.yaw _returnvalue) (.yaw _returnvalue_2)))
  (bind _returnvalue_4 (Math|Float|ClampAngle _returnvalue_3 -179.9 -1.8e+02))
  (bind _asbp_player_animation (Utilities|Casting|CastToBP_Player_Animation (Components|SkeletalMesh|GetAnimInstance (Variables|Character|GetMesh))))
  (Variables|/Game/Blueprints/Player/BP_Player_Animation.BP_Player_Animation_C|SetHeadRotation _asbp_player_animation (Math|Rotator|MakeRotator (- 0.0 (.pitch _returnvalue)) 0.0 _returnvalue_4))
  (if (> _returnvalue_4 9e+01)
    (Variables|Default|SetYawOffset 9e+01)
    (Variables|Default|SetActorYaw (+ (.yaw (Transformation|GetActorRotation)) (Variables|Default|GetYawOffset)) :!label _label)
    (Transformation|SetActorRotation (Math|Interpolation|RInterpTo (Transformation|GetActorRotation) (Math|Rotator|MakeRotator 0.0 0.0 (Variables|Default|GetActorYaw)) (Utilities|Time|GetWorldDeltaSeconds) 5.0))
    (elif (< _returnvalue_4 -9e+01)
      (Variables|Default|SetYawOffset -9e+01)
      (goto _label))))

(fn PickupItem
  (params (ClassRef :type Actor%20Object%20Reference)))