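; Door actor that the player swings open or shut by holding the DragDoor input and turning.
; On press, a line trace from the player camera checks for any BP_Door, not specifically this instance.
; While held, Tick rotates the Arrow component by the player's TurnRate times Sensitivity.
; When its world yaw falls outside the Angle-based clamp, it resets relative yaw to one degree off Angle.
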(event EventBeginPlay
  (Input|EnableInput (Game|GetPlayerController 0)))

(event EventTick
  (params (DeltaSeconds :type Float%20%28single-precision%29))
  (bind _angle (Variables|Default|GetAngle))
  (bind _arrow (Variables|Default|GetArrow))
  (bind _arrow_2 (Variables|Default|GetArrow))
  (bind _angle_2 (Variables|Default|GetAngle))
  (bind _returnvalue (Transformation|GetWorldRotation _arrow))
  (if (Variables|Default|GetIsHoldingLMB)
    (if (Variables|Default|GetIsLookingAtDoor)
      (if (not (== (.yaw _returnvalue) (Math|Float|ClampAngle (.yaw _returnvalue) _angle (* _angle -1.0))))
        (Transformation|AddLocalRotation _arrow_2 (Math|Rotator|MakeRotator 0.0 0.0 (* (Variables|/Game/Blueprints/Player/BP_Player.BP_Player_C|GetTurnRate (stale Input|ActionEvents|InputActionDragDoor _asbp_player)) (Variables|Default|GetSensitivity))) false false)
        (elif (>= (.yaw _returnvalue) _angle_2)
          (Transformation|SetRelativeRotation _arrow_2 (Math|Rotator|MakeRotator 0.0 0.0 (- _angle_2 1.0)) false false)
          (else
            (Transformation|SetRelativeRotation _arrow_2 (Math|Rotator|MakeRotator 0.0 0.0 (+ (* _angle_2 1.0) 1.0)) false false)))))))

(event Input|ActionEvents|InputActionDragDoor
  (params (Key :type Key%20Structure :default "None"))
  (:Pressed
    (Variables|Default|SetIsHoldingLMB true)
    (bind _asbp_player (Utilities|Casting|CastToBP_Player (Game|GetPlayerCharacter 0)))
    (bind (_outhit _returnvalue) (Collision|LineTraceForObjects (Transformation|GetWorldLocation (Variables|/Game/Blueprints/Player/BP_Player.BP_Player_C|GetCamera _asbp_player)) (+ (Transformation|GetWorldLocation (Variables|/Game/Blueprints/Player/BP_Player.BP_Player_C|GetCamera _asbp_player)) (* (Math|Vector|GetForwardVector (Variables|/Game/Blueprints/Player/BP_Player.BP_Player_C|GetCamera _asbp_player)) 5e+02)) (Utilities|Array|MakeArray "ObjectTypeQuery2") false 0 "None" false))
    (if _returnvalue
      (Utilities|Casting|CastToBP_Door (.HitActor (Collision|BreakHitResult _outhit)))
      (Variables|Default|SetIsLookingAtDoor true)
      (else
        (Variables|Default|SetIsLookingAtDoor false))))
  (:Released
    (Variables|Default|SetIsHoldingLMB false)))

(fn ConstructionScript)